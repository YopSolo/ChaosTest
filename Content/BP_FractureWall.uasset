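; BP_FractureWall is a destructible Chaos wall that shatters when a rolling third-person character hits it.
; On box overlap by a rolling character, it moves a referenced Chaos field to the character's Y position and triggers it.
; The Geometry Collection's break event plays a world camera shake at the wall and, through a DoOnce, briefly slows global time on the first break only.
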(event `self.Box.OnComponentBeginOverlap`
  (params (OverlappedComponent :type "PrimitiveComponent Object Reference") (OtherActor :type "Actor Object Reference") (OtherComp :type "PrimitiveComponent Object Reference") (OtherBodyIndex :type Integer) (bFromSweep :type Boolean) (SweepResult :type "HitResult Structure (by ref)"))
  (bind _chaosfield (`self.ChaosField`))
  (bind (_returnvalue_x _returnvalue_y _returnvalue_z) (`KismetMathLibrary.BreakVector` (`self.K2_GetActorLocation` _chaosfield)))
  (bind _asbp_third_person_character (cast `/Game/ThirdPerson/Blueprints/BP_ThirdPersonCharacter` OtherActor))
  (if (`/Game/ThirdPerson/Blueprints/BP_ThirdPersonCharacter.isRolling?` _asbp_third_person_character)
    (`/Engine/EditorBlueprintResources/StandardMacros.IsValid` (`self.ChaosField`)
      (:`Is Valid`
        (bind (_returnvalue_x_2 _returnvalue_y_2) (`KismetMathLibrary.BreakVector` (`self.K2_GetActorLocation` _asbp_third_person_character)))
        (`self.K2_SetActorLocation` _chaosfield (`KismetMathLibrary.MakeVector` _returnvalue_x _returnvalue_y_2 _returnvalue_z) false true)
        (`/Engine/EditorResources/FieldNodes/FS_MasterField.CE_Trigger` (`self.ChaosField`))))))

(event `self.GeometryCollection.OnChaosBreakEvent`
  (params (BreakEvent :type "ChaosBreakEvent Structure (by ref)"))
  (`|ExecutionSequence`
    (:`then_0`
      (`/Engine/EditorBlueprintResources/StandardMacros.DoOnce` false
        (:`Completed`
          (`GameplayStatics.SetGlobalTimeDilation` 0.3)
          (`KismetSystemLibrary.Delay` 0.5)
          (`GameplayStatics.SetGlobalTimeDilation` 1.0))))
    (:`then_1`
      (`GameplayStatics.PlayWorldCameraShake` "/Game/BP_MyCamShake.BP_MyCamShake_C" (`self.K2_GetActorLocation`) 10.0 1000.0))))

(fn `UserConstructionScript`)